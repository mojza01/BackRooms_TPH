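; BP_Monster is an AI enemy that roams, chases the first-person player on sight and ends the game when it catches them.
; Roaming loops between random reachable nearby points with short pauses.
; PawnSensing sightings start a move to the player's current location, and a retriggerable delay resumes roaming once sightings stop.
; Player overlap with AttackZone shows the game-over widget, switches to UI input and freezes the game.
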(event OnSeePawn(PawnSensing)
  (params (Pawn :type Pawn%20Object%20Reference))
  (Variables|Default|SetIsChasing true)
  (bind _asbp_first_person_character (Utilities|Casting|CastToBP_FirstPersonCharacter Pawn))
  (Variables|Default|SetTargetPlayer _asbp_first_person_character)
  (AI|AIMoveTo self (Transformation|GetActorLocation (Variables|Default|GetTargetPlayer)) 0 75.0 false
    (:then
      (Utilities|FlowControl|RetriggerableDelay 3.0)
      (Variables|Default|SetIsChasing false)
      (CallFunction|StartRoaming))))

(event OnComponentBeginOverlap(AttackZone)
  (params (OverlappedComponent :type Primitive%20Component%20Object%20Reference) (OtherActor :type Actor%20Object%20Reference) (OtherComp :type Primitive%20Component%20Object%20Reference) (OtherBodyIndex :type Integer) (bFromSweep :type Boolean) (SweepResult :type Hit%20Result%20Structure%20%28by%20ref%29))
  (Utilities|Casting|CastToBP_FirstPersonCharacter OtherActor)
  (bind _returnvalue (UserInterface|CreateWidget "/Game/RandalSource/AI/WBP_GameOver.WBP_GameOver_C"))
  (UserInterface|Viewport|AddtoViewport _returnvalue 0)
  (Variables|/Script/Engine.PlayerController|SetbShowMouseCursor (Game|GetPlayerController 0) true)
  (Input|SetInputModeUIOnly (Game|GetPlayerController 0) _returnvalue "DoNotLock" false)
  (Game|SetGamePaused true)
  (Utilities|Time|SetGlobalTimeDilation 0.0))

(event Custom|StartRoaming
  (if (not (Variables|Default|GetIsChasing))
    (AI|AIMoveTo self (.RandomLocation (AI|Navigation|GetRandomReachablePointinRadius (Transformation|GetActorLocation) 2e+03 0 0)) 0 75.0 false
      (:OnSuccess
        (Utilities|FlowControl|Delay 2.0)
        (CallFunction|StartRoaming))
      (:OnFail
        (Utilities|FlowControl|Delay 2.0)
        (CallFunction|StartRoaming)))))

(event Collision|EventActorBeginOverlap
  (params (OtherActor :type Actor%20Object%20Reference)))

(event EventTick
  (params (DeltaSeconds :type Float%20%28single-precision%29)))

(event EventBeginPlay
  (CallFunction|StartRoaming))

(fn ConstructionScript)